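; Tutorial game mode that lays out a random chain of road, master, train track and river tiles at BeginPlay.
; It calls SpawnTile a fixed number of times, each picking a tile class at random, with roads weighted double.
; Each new tile's SpawnPoint world location becomes NextSpawnPoint for the following one, with rotation and scale reset, so tiles connect end to end.
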(event `self.ReceiveBeginPlay`
  (for _ (range 15)
    (`self.SpawnTile`)))

(fn `SpawnTile`
  (switch `int` (`KismetMathLibrary.RandomIntegerInRange` 0 4)
    (:`0`
      (bind _returnvalue (`|SpawnActorFromClass` "/Game/Blueprints/Map_Assets_BP/roads_BP/road_L_R.road_L_R_C" (`self.NextSpawnPoint`) "Undefined" "OverrideRootScale" null null :!label _label))
      (bind _asroad_l_r (cast `/Game/Blueprints/Map_Assets_BP/roads_BP/road_L_R` _returnvalue))
      (set `self.NextSpawnPoint` (`KismetMathLibrary.MakeTransform` (`SceneComponent.K2_GetComponentLocation` (`/Game/Blueprints/Map_Assets_BP/roads_BP/road_L_R.SpawnPoint` _asroad_l_r)))))
    (:`1`
      (goto _label))
    (:`2`
      (bind _returnvalue_2 (`|SpawnActorFromClass` "/Game/Blueprints/Map_Assets_BP/roads_BP/MasterTile.MasterTile_C" (`self.NextSpawnPoint`) "Undefined" "OverrideRootScale" null null))
      (bind _asmaster_tile (cast `/Game/Blueprints/Map_Assets_BP/roads_BP/MasterTile` _returnvalue_2))
      (set `self.NextSpawnPoint` (`KismetMathLibrary.MakeTransform` (`SceneComponent.K2_GetComponentLocation` (`/Game/Blueprints/Map_Assets_BP/roads_BP/MasterTile.SpawnPoint` _asmaster_tile)))))
    (:`3`
      (bind _returnvalue_3 (`|SpawnActorFromClass` "/Game/Blueprints/Map_Assets_BP/roads_BP/TrainTrack.TrainTrack_C" (`self.NextSpawnPoint`) "Undefined" "OverrideRootScale" null null))
      (bind _astrain_track (cast `/Game/Blueprints/Map_Assets_BP/roads_BP/TrainTrack` _returnvalue_3))
      (set `self.NextSpawnPoint` (`KismetMathLibrary.MakeTransform` (`SceneComponent.K2_GetComponentLocation` (`/Game/Blueprints/Map_Assets_BP/roads_BP/TrainTrack.SpawnPoint` _astrain_track)))))
    (:`4`
      (bind _returnvalue_4 (`|SpawnActorFromClass` "/Game/Blueprints/Map_Assets_BP/roads_BP/river_L_R1.river_L_R1_C" (`self.NextSpawnPoint`) "Undefined" "OverrideRootScale" null null))
      (bind _asriver_l_r1 (cast `/Game/Blueprints/Map_Assets_BP/roads_BP/river_L_R1` _returnvalue_4))
      (set `self.NextSpawnPoint` (`KismetMathLibrary.MakeTransform` (`SceneComponent.K2_GetComponentLocation` (`/Game/Blueprints/Map_Assets_BP/roads_BP/river_L_R1.SpawnPoint` _asriver_l_r1)))))))

(fn `UserConstructionScript`)